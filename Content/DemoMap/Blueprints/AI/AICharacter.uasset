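; AI character Blueprint that works with a SampleAIController to track a target actor and face it.
; On possession it caches the controller and listens for target changes to update its current target.
; SetCanAttackAndTarget writes the CanAttack blackboard key and passes the target to the controller.
; GetDesiredRotation returns a yaw-only look-at toward the target, or the current rotation when there is none.
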(event `self.ReceivePossessed`
  (params (NewController :type "Controller Object Reference"))
  ;[0 0.03342 1] Store Controller on posses
  (bind _assample_aicontroller (cast `/Game/DemoMap/Blueprints/AI/SampleAIController` NewController))
  (bind _output_get (set `self.AIController` _assample_aicontroller))
  (add `/Game/DemoMap/Blueprints/AI/SampleAIController.OnTargetActorChanged` _output_get (delegate `OnTargetActorChanged_Event_0`)))

(event `OnTargetActorChanged_Event_0`
  (params (NewTargetActor :type "Actor Object Reference"))
  (set `self.CurrentTargetActor` NewTargetActor))

(event `SetCanAttackAndTarget`
  (params (Value :type Boolean) (Target :type "Actor Object Reference"))
  ;[0 0.03342 1] Update Can Attack And Target in blackboard
  (bind _aicontroller (`self.AIController`)
    (:`then`
      (`BlackboardComponent.SetValueAsBool` (`AIController.Blackboard` _aicontroller) "CanAttack" Value)
      (`/Game/DemoMap/Blueprints/AI/SampleAIController.SetTargetActor` _aicontroller Target))
    (:`else`)))

(fn `GetDesiredRotation`
  (returns (ReturnValue :type "Rotator Structure"))
  (bind _currenttargetactor (`self.CurrentTargetActor`)
    (:`then`
      ;[1 1 1] Return rotation towards selected target
      (return (`KismetMathLibrary.MakeRotator` (.roll (`self.K2_GetActorRotation`)) (.pitch (`self.K2_GetActorRotation`)) (.yaw (`KismetMathLibrary.FindLookAtRotation` (`self.K2_GetActorLocation`) (`self.K2_GetActorLocation` _currenttargetactor))))))
    (:`else`
      ;[1 1 1] Return actor rotation means no rotate at all
      (return (`self.K2_GetActorRotation`)))))

(fn `UserConstructionScript`
  (`parent.UserConstructionScript`))