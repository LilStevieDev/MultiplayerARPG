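; AI controller for the demo map's sample AI, which runs the BT_SampleAI behavior tree and targets the player.
; On BeginPlay, once the tree starts, it stores the pawn's location as SpawnLocation in the blackboard and sets player character 0 as Target.
; SetTargetActor updates the target only on change, fires a target-changed call and writes it to the blackboard.
; An OnRep handler mirrors a valid replicated Target into the blackboard.
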(event `self.ReceiveBeginPlay`
  ;[0 0.03342 1] Run Behavior Tree
  (bind _returnvalue (`self.RunBehaviorTree` "/Game/DemoMap/Blueprints/AI/BT_SampleAI.BT_SampleAI"))
  (if _returnvalue
    ;[0 0.03342 1] Set SpawnLocation value in blackboard
    (`BlackboardComponent.SetValueAsVector` (`self.Blackboard`) "SpawnLocation" (`self.K2_GetActorLocation` (`self.K2_GetPawn`)))
    ;[0 0.03342 1] Set Player Character as target in blackboard
    (`self.SetTargetActor` (`GameplayStatics.GetPlayerCharacter` 0))))

(fn `OnRep_Target`
  (bind _target (`self.Target`)
    (:`then`
      (`BlackboardComponent.SetValueAsObject` (`self.Blackboard`) "Target" _target))
    (:`else`)))

(fn `SetTargetActor`
  (params (NewTarget :type "Actor Object Reference"))
  (if (!= NewTarget (`self.Target`))
    (bind _output_get (set `self.Target` NewTarget))
    (`self.OnTargetActorChanged` _output_get)
    (`BlackboardComponent.SetValueAsObject` (`self.Blackboard`) "Target" _output_get)))

(fn `UserConstructionScript`)