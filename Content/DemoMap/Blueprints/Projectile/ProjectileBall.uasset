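; ProjectileBall is a demo projectile that deals fixed damage to what it hits, credited to its owner's instigator.
; On BeginPlay it copies the owner's collision debug setting, ignores the owner, sets a limited lifespan and activates CCCollisionHandler tracing on the sphere mesh's sockets.
; On hit it deactivates that collision, applies damage and switches the sphere to a simulated Ragdoll-profile body.
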(event `SetupDebug`
  ;[0 0.03342 1] Setup Debug
  (set `CCCollisionHandlerComponent.bDebug` (`CCCollisionHandlerComponent.bDebug` (`self.GetComponentByClass` (`self.GetOwner`) "/Script/CombatComponents.CCCollisionHandlerComponent")) (`self.CCCollisionHandler`)))

(event `self.ReceiveBeginPlay`
  (bind _sphere (`self.Sphere`))
  (`self.SetupDebug`)
  (`self.SetLifeSpan` 10.0) ; auto destroy after 10 secs\nif projectile didnt\nhit anything
  ;[0 0.03342 1] Always ignore owner
  (`KismetArrayLibrary.Array_Add` (`CCCollisionHandlerComponent.IgnoredActors` (`self.CCCollisionHandler`)) (`self.GetOwner`))
  ;[0 0.03342 1] Set ball sphere mesh as colliding object and activate collision
  (`CCCollisionHandlerComponent.UpdateCollidingComponent` (`self.CCCollisionHandler`) _sphere (`SceneComponent.GetAllSocketNames` _sphere))
  (`CCCollisionHandlerComponent.ActivateCollision` (`self.CCCollisionHandler`) "NONE"))

(event `self.CCCollisionHandler.OnHit`
  (params (HitResult :type "HitResult Structure (by ref)") (CollidingComponent :type "PrimitiveComponent Object Reference"))
  ;[0 0.03342 1] On Hit make sure it wasn't owner, and print out hit actor name
  (`CCCollisionHandlerComponent.DeactivateCollision` (`self.CCCollisionHandler`))
  (`self.EnablePhysics`)
  (`GameplayStatics.ApplyDamage` (`.HitActor` (`GameplayStatics.BreakHitResult` HitResult)) 20.0 (`self.GetInstigatorController` (`self.GetOwner`)) self))

(event `EnablePhysics`
  (bind _sphere (`self.Sphere`))
  (`PrimitiveComponent.SetCollisionProfileName` _sphere "Ragdoll" true)
  (`PrimitiveComponent.SetSimulatePhysics` _sphere true))

(fn `UserConstructionScript`)