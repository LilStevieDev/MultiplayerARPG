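; Base character for the DemoMap: networked combat with sword, dual-sword, hand and thrown-ball attacks, plus rolling.
; Server events gate actions through CanPerformAction, then multicast montages and weapon socket attachments; delays based on montage length clear state flags.
; CCCollisionHandler traces the active weapon or arm sockets and applies damage on hit.
; Health RepNotify updates the widget bar and triggers ragdoll death; GetDesiredRotation turns attacks and rolls toward movement input.
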(event `Server_PlayMontageSection`
  (params (MontageToPlay :type "AnimMontage Object Reference") (StartSectionName :type Name))
  ;[0 0.03342 1] Helper Events
  ; *Play Montage
  ; *Set Debug
  ; *Update Health Widget
  (`self.Net_PlayMontageSection` MontageToPlay StartSectionName))

(event `Net_PlayMontageSection`
  (params (MontageToPlay :type "AnimMontage Object Reference") (StartSectionName :type Name))
  ;[0 0.03342 1] Helper Events
  ; *Play Montage
  ; *Set Debug
  ; *Update Health Widget
  (bind _returnvalue (`self.PlayAnimMontage` MontageToPlay 1.0 StartSectionName))
  (set `self.MontageDuration` _returnvalue))

(event `Server_PlayMontage`
  (params (MontageToPlay :type "AnimMontage Object Reference"))
  ;[0 0.03342 1] Helper Events
  ; *Play Montage
  ; *Set Debug
  ; *Update Health Widget
  (`self.Net_PlayMontage` MontageToPlay))

(event `Net_PlayMontage`
  (params (MontageToPlay :type "AnimMontage Object Reference"))
  ;[0 0.03342 1] Helper Events
  ; *Play Montage
  ; *Set Debug
  ; *Update Health Widget
  (bind _returnvalue (`AnimInstance.Montage_Play` (`SkeletalMeshComponent.GetAnimInstance` (`self.Mesh`)) MontageToPlay 1.0 "Duration" 0.0 true))
  (set `self.MontageDuration` _returnvalue))

(event `Server_ToggleAttackingAI`
  (params (AIChar :type "/Game/DemoMap/Blueprints/AI/AICharacter Object Reference") (Value :type Boolean))
  ;[0 0.03342 1] Helper Events
  ; *Play Montage
  ; *Set Debug
  ; *Update Health Widget
  (`/Engine/EditorBlueprintResources/StandardMacros.IsValid` AIChar
    (:`Is Valid`
      (`/Game/DemoMap/Blueprints/AI/AICharacter.SetCanAttackAndTarget` AIChar Value self))))

(event `SetDebug`
  (params (bDebug :type Boolean))
  ;[0 0.03342 1] Helper Events
  ; *Play Montage
  ; *Set Debug
  ; *Update Health Widget
  (set `CCCollisionHandlerComponent.bDebug` bDebug (`self.CCCollisionHandler`)))

(event `UpdateHealthBar`
  ;[0 0.03342 1] Helper Events
  ; *Play Montage
  ; *Set Debug
  ; *Update Health Widget
  (bind _aswb_health_bar (cast `/Game/DemoMap/Blueprints/WB_HealthBar` (`WidgetComponent.GetUserWidgetObject` (`self.HealthWidget`))))
  (`ProgressBar.SetPercent` (`/Game/DemoMap/Blueprints/WB_HealthBar.HealthProgressBar` _aswb_health_bar) (/ (`self.Health`) (`self.MaxHealth`))))

(event `Server_AttackPressed`
  ;[0 0.03342 1] Character actions Events
  ; *Attack
  ; *Roll
  ; *Change Combat Mode
  (`self.CanPerformAction`
    (:`true`
      (switch `/Game/DemoMap/Blueprints/E_CombatMode` (`self.CombatMode`)
        (:`NewEnumerator0`
          (set `self.SelectedAttackMontage` "/Game/DemoMap/Mannequin/Animations/SwordAttack_Montage.SwordAttack_Montage")
          (`self.Server_PlayMontage` (`self.SelectedAttackMontage`) :!label _label)
          (set `self.IsAttacking` true)
          (`KismetSystemLibrary.Delay` (* (`self.MontageDuration`) 0.8))
          (set `self.IsAttacking` false))
        (:`NewEnumerator1`
          (set `self.SelectedAttackMontage` "/Game/DemoMap/Mannequin/Animations/DualSwordAttack_Montage.DualSwordAttack_Montage")
          (goto _label))
        (:`NewEnumerator2`
          (set `self.SelectedAttackMontage` "/Game/DemoMap/Mannequin/Animations/HandsAttack_Montage.HandsAttack_Montage")
          (goto _label))
        (:`NewEnumerator3`
          (`self.Server_PlayMontageSection` "/Game/DemoMap/Mannequin/Animations/Throwing_Montage.Throwing_Montage" "Start")
          (set `self.IsThrowing` true))))))

(event `Server_Roll`
  ;[0 0.03342 1] Character actions Events
  ; *Attack
  ; *Roll
  ; *Change Combat Mode
  (`self.CanPerformAction`
    (:`true`
      (`self.Server_PlayMontage` "/Game/DemoMap/Mannequin/Animations/Roll_Montage.Roll_Montage")
      (set `self.IsRolling` true)
      (`KismetSystemLibrary.Delay` (* (`self.MontageDuration`) 0.8))
      (set `self.IsRolling` false))))

(event `Server_AttackReleased`
  ;[0 0.03342 1] Character actions Events
  ; *Attack
  ; *Roll
  ; *Change Combat Mode
  (switch `/Game/DemoMap/Blueprints/E_CombatMode` (`self.CombatMode`)
    (:`NewEnumerator3`
      (if (`self.IsThrowing`)
        (`self.Server_PlayMontageSection` "/Game/DemoMap/Mannequin/Animations/Throwing_Montage.Throwing_Montage" "Throw")
        (`|SpawnActorFromClass` "/Game/DemoMap/Blueprints/Projectile/ProjectileBall.ProjectileBall_C" (`KismetMathLibrary.MakeTransform` (`SceneComponent.K2_GetComponentLocation` (`self.BallSpawn`)) (`self.K2_GetActorRotation`)) "AlwaysSpawn" "OverrideRootScale" self (`CCCollisionHandlerComponent.bDebug` (`self.CCCollisionHandler`)) self)
        (`KismetSystemLibrary.Delay` 0.3)
        (set `self.IsThrowing` false)))))

(event `Server_SetCombatMode`
  (params (NewCombatMode :type "/Game/DemoMap/Blueprints/E_CombatMode Enum" :default "NewEnumerator0"))
  ;[0 0.03342 1] Character actions Events
  ; *Attack
  ; *Roll
  ; *Change Combat Mode
  (`self.CanPerformAction`
    (:`true`
      (bind _output_get (set `self.CombatMode` NewCombatMode))
      (switch `/Game/DemoMap/Blueprints/E_CombatMode` _output_get
        (:`NewEnumerator0`
          (`self.Server_AttachToMesh` (`self.LeftHandSword`) "left_back_sword")
          (`self.Server_AttachToMesh` (`self.RightHandSword`) "right_hand_sword"))
        (:`NewEnumerator1`
          (`self.Server_AttachToMesh` (`self.LeftHandSword`) "left_hand_sword")
          (`self.Server_AttachToMesh` (`self.RightHandSword`) "right_hand_sword"))
        (:`NewEnumerator2`
          (`self.Server_AttachToMesh` (`self.LeftHandSword`) "left_back_sword" :!label _label_2)
          (`self.Server_AttachToMesh` (`self.RightHandSword`) "right_back_sword"))
        (:`NewEnumerator3`
          (goto _label_2))))))

(event `Server_AttachToMesh`
  (params (Component :type "SceneComponent Object Reference") (SocketName :type Name))
  ;[0 0.03342 1] Character actions Events
  ; *Attack
  ; *Roll
  ; *Change Combat Mode
  (`self.Net_AttachToMesh` Component SocketName))

(event `Net_AttachToMesh`
  (params (Component :type "SceneComponent Object Reference") (SocketName :type Name))
  ;[0 0.03342 1] Character actions Events
  ; *Attack
  ; *Roll
  ; *Change Combat Mode
  (`SceneComponent.K2_AttachToComponent` Component (`self.Mesh`) SocketName "KeepRelative" "KeepRelative" "KeepRelative" true))

(event `Server_Death`
  (bind _returnvalue (`self.GetController`))
  ;[0 0.03342 1] Received Damage Events
  ; *AnyDamage
  ; *Death
  (`/Engine/EditorBlueprintResources/StandardMacros.IsValid` _returnvalue
    (:`Is Valid`
      (`Controller.UnPossess` _returnvalue))
    (:`Is Not Valid`
      _))
  (`self.Net_Death`)
  (`self.SetLifeSpan` 5.0))

(event `self.ReceiveAnyDamage`
  (params (Damage :type "Float (single-precision)") (DamageType :type "DamageType Object Reference") (InstigatedBy :type "Controller Object Reference") (DamageCauser :type "Actor Object Reference"))
  ;[0 0.03342 1] Received Damage Events
  ; *AnyDamage
  ; *Death
  (set `self.Health` (- (`self.Health`) Damage)))

(event `Net_Death`
  (bind _mesh (`self.Mesh`))
  ;[0 0.03342 1] Received Damage Events
  ; *AnyDamage
  ; *Death
  (`PrimitiveComponent.SetCollisionProfileName` _mesh "Ragdoll" true)
  (`PrimitiveComponent.SetSimulatePhysics` _mesh true)
  (`PrimitiveComponent.SetCollisionEnabled` (`self.CapsuleComponent`) "NoCollision")
  (`SceneComponent.SetVisibility` (`self.HealthWidget`) false false))

(event `self.ReceiveBeginPlay`
  ;[0 0.03342 1] Begin Play
  ; If controlled locally, set combat mode
  (`self.IsLocallyControlled`
    (:`True`
      (`self.Server_SetCombatMode` "NewEnumerator1"))))

(event `self.CCRotatingOwner.OnRotatingStart`
  ;[0 0.03342 1] Rotation Owner Events
  ; *On Rotating Start
  ; *On Rotating End
)

(event `self.CCRotatingOwner.OnRotatingEnd`
  ;[0 0.03342 1] Rotation Owner Events
  ; *On Rotating Start
  ; *On Rotating End
)

(event `self.CCCollisionHandler.OnCollisionActivated`
  (params (CollisionPart :type "ECCCollisionPart Enum" :default "NONE"))
  (bind _righthandsword (`self.RightHandSword`))
  (bind _lefthandsword (`self.LeftHandSword`))
  (bind _righthandsword_2 (`self.RightHandSword`))
  (bind _lefthandsword_2 (`self.LeftHandSword`))
  ;[0 0.03342 1] Collision Handler Events
  ; *On Activated
  ; *On Deactivated
  ; *On Hit
  (switch `ECCCollisionPart` CollisionPart
    (:`PrimaryItem`
      (`CCCollisionHandlerComponent.UpdateCollidingComponent` (`self.CCCollisionHandler`) _righthandsword (`SceneComponent.GetAllSocketNames` _righthandsword)))
    (:`SecondaryItem`
      (`CCCollisionHandlerComponent.UpdateCollidingComponent` (`self.CCCollisionHandler`) _lefthandsword_2 (`SceneComponent.GetAllSocketNames` _lefthandsword_2)))
    (:`BothHandItems`
      (`CCCollisionHandlerComponent.UpdateCollidingComponents` (`self.CCCollisionHandler`) (`|MakeArray` (make `CCCollidingComponent` _righthandsword_2 (`SceneComponent.GetAllSocketNames` _righthandsword_2)) (make `CCCollidingComponent` _lefthandsword (`SceneComponent.GetAllSocketNames` _lefthandsword)))))
    (:`RightArm`
      (`CCCollisionHandlerComponent.UpdateCollidingComponent` (`self.CCCollisionHandler`) (`self.Mesh`) (`self.RightHandCollisionSockets`)))))

(event `self.CCCollisionHandler.OnCollisionDeactivated`
  ;[0 0.03342 1] Collision Handler Events
  ; *On Activated
  ; *On Deactivated
  ; *On Hit
)

(event `self.CCCollisionHandler.OnHit`
  (params (HitResult :type "HitResult Structure (by ref)") (CollidingComponent :type "PrimitiveComponent Object Reference"))
  ;[0 0.03342 1] Collision Handler Events
  ; *On Activated
  ; *On Deactivated
  ; *On Hit
  (`GameplayStatics.ApplyDamage` (`.HitActor` (`GameplayStatics.BreakHitResult` HitResult)) (`self.Damage`) (`self.GetController`) self))

(fn `CanJumpInternal`
  (returns (ReturnValue :type Boolean))
  (`self.CanPerformAction`
    (:`true`
      (bind _returnvalue (`parent.CanJumpInternal`))
      (return _returnvalue))
    (:`false`
      (return false))))

(fn `GetDesiredRotation`
  (returns (ReturnValue :type "Rotator Structure"))
  ;[0 0.03342 1] is attacking or rolling
  (if (or (`self.IsAttacking`) (`self.IsRolling`))
    ;[0 0.03342 1] Has any movement input (any movement input pressed)
    (if (!= (`CharacterMovementComponent.GetCurrentAcceleration` (`self.CharacterMovement`)) (0.0 0.0 0.0))
      ;[0 0.03342 1] Use yaw from input movement means rotate towards input
      (return (`KismetMathLibrary.MakeRotator` (.roll (`self.K2_GetActorRotation`)) (.pitch (`self.K2_GetActorRotation`)) (.yaw (`KismetMathLibrary.Conv_VectorToRotator` (`CharacterMovementComponent.GetCurrentAcceleration` (`self.CharacterMovement`))))))
      (else
        _)))
  ;[0 0.03342 1] return actor rotation means dont rotate at all
  (return (`self.K2_GetActorRotation`)))

(fn `OnRep_Health`
  ;[0 0.03342 1] Whenever health change, update health progress bar and check if character is still alive
  (`self.UpdateHealthBar`)
  (if (<= (`self.Health`) 0.0)
    (`/Engine/EditorBlueprintResources/ActorMacros.Switch Has Authority`
      (:`Authority`
        (`self.Server_Death`)))))

(fn `UserConstructionScript`)